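; BP_Door is a door actor that swings open and closed when its Interaction event fires.
; A FlipFlop alternates between playing and reversing the DoorAction timeline, whose play rate is set from Speed on BeginPlay.
; The timeline track is mapped to a yaw of up to Angle on the static mesh, keeping its current roll and pitch.
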(event EventInteraction
  (params (Mesh :type Static%20Mesh%20Object%20Reference) (Tab :type Array%20of%20Struc%20Inventory%20Structures))
  (bind _staticmesh (Variables|Default|GetStaticMesh))
  (bind _relativerotation (Variables|/Script/Engine.SceneComponent|GetRelativeRotation _staticmesh))
  (Utilities|FlowControl|FlipFlop
    (:A
      (bind _newtrack_0 (Timeline|DoorAction Play)
        (:Update
          (Transformation|SetRelativeRotation _staticmesh (Math|Rotator|MakeRotator (.roll _relativerotation) (.pitch _relativerotation) (Math|Float|MapRangeClamped _newtrack_0 0.0 1.0 0.0 (Variables|Default|GetAngle))) false false))))
    (:B
      (Timeline|DoorAction Reverse))))

(event EventBeginPlay
  (Components|Timeline|SetPlayRate (Variables|Default|GetDoorAction) (Variables|Default|GetSpeed)))

(fn ConstructionScript
  (|CallParentFunction))