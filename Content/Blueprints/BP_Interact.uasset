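; BP_Interact is an interactable object with a configurable static mesh and material, applied in the construction script.
; RenderDepthON and RenderDepthOFF toggle custom depth rendering on the mesh.
; Interact only prints a debug string, and PreviewAction takes a mesh but has no implementation.
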(event Custom|Render%20Depth%20OFF
  (Rendering|SetRenderCustomDepth (Variables|Default|GetStaticMesh) false))

(event Custom|Render%20Depth%20ON
  (Rendering|SetRenderCustomDepth (Variables|Default|GetStaticMesh) true))

(event Custom|PreviewAction
  (params (Mesh :type Static%20Mesh%20Object%20Reference)))

(event Custom|Interact
  (Development|PrintString "Interaction"))

(fn ConstructionScript
  (bind _staticmesh (Variables|Default|GetStaticMesh))
  (Components|StaticMesh|SetStaticMesh _staticmesh (Variables|Default|GetMesh))
  (Rendering|Material|SetMaterial _staticmesh 0 (Variables|Default|GetMaterial)))