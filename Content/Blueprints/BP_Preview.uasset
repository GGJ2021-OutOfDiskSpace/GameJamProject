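; BP_Preview is a preview actor that can be filled once with a supplied mesh.
; It starts with its StaticMesh collision object type set to Visibility.
; On PreviewAction, if unused and given a valid mesh, it marks itself used, switches to WorldDynamic, takes that mesh and its first material, and removes the first entry from the passed Tab array.
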(event EventBeginPlay
  (Collision|SetCollisionObjectType (Variables|Default|GetStaticMesh) "ECC_Visibility"))

(event EventPreviewAction
  (params (Mesh :type Static%20Mesh%20Object%20Reference) (Tab :type Array%20of%20Struc%20Inventory%20Structures))
  (bind _staticmesh (Variables|Default|GetStaticMesh))
  (if (not (Variables|Default|GetUse))
    (Utilities|IsValid Mesh
      (:Is%20Valid
        (Variables|Default|SetUse true)
        (Collision|SetCollisionObjectType (Variables|Default|GetStaticMesh) "ECC_WorldDynamic")
        (Rendering|Material|SetMaterial _staticmesh 0 (Rendering|Material|GetMaterial Mesh 0))
        (Components|StaticMesh|SetStaticMesh _staticmesh Mesh)
        (Utilities|Array|RemoveIndex Tab)))))

(fn ConstructionScript
  (|CallParentFunction))