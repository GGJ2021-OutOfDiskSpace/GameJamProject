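; Piano actor that plays a sound when interacted with while the BP_PetitFille character is near it.
; Box overlap begin and end toggle a can-use flag for that character, which gates the Interaction event.
; Interaction lazily creates a reusable 2D audio component from SoundToPlay and starts it only if it is not already playing.
; Leaving the box does not stop playback.
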(event OnComponentBeginOverlap(Box)
  (params (OverlappedComponent :type Primitive%20Component%20Object%20Reference) (OtherActor :type Actor%20Object%20Reference) (OtherComp :type Primitive%20Component%20Object%20Reference) (OtherBodyIndex :type Integer) (bFromSweep :type Boolean) (SweepResult :type Hit%20Result%20Structure%20%28by%20ref%29))
  (Utilities|Casting|CastToBP_PetitFille OtherActor)
  (Variables|Default|SetsetCanUse? true))

(event OnComponentEndOverlap(Box)
  (params (OverlappedComponent :type Primitive%20Component%20Object%20Reference) (OtherActor :type Actor%20Object%20Reference) (OtherComp :type Primitive%20Component%20Object%20Reference) (OtherBodyIndex :type Integer))
  (Utilities|Casting|CastToBP_PetitFille OtherActor)
  (Variables|Default|SetsetCanUse? false))

(event EventBeginPlay)

(event Collision|EventActorBeginOverlap
  (params (OtherActor :type Actor%20Object%20Reference)))

(event EventTick
  (params (DeltaSeconds :type Float%20%28single-precision%29)))

(event EventInteraction
  (params (Tab :type Array%20of%20Struc%20Inventory%20Structures))
  (if (Variables|Default|GetsetCanUse?)
    (Utilities|IsValid (Variables|Default|GetAudioToPlay)
      (:Is%20Valid
        _)
      (:Is%20Not%20Valid
        (bind _returnvalue (Audio|CreateSound2D (Variables|Default|GetSoundToPlay) 1.0 1.0 0.0 0))
        (Variables|Default|SetAudioToPlay _returnvalue)))
    (if (not (Audio|Components|Audio|IsPlaying (Variables|Default|GetAudioToPlay)))
      (Audio|Components|Audio|Play (Variables|Default|GetAudioToPlay) 0.0))))

(fn ConstructionScript
  (|CallParentFunction))