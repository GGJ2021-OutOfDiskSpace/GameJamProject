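; BP_SoundEvent is a one-shot trigger volume that plays a scripted sequence of sounds when the BP_PetitFille character enters its box.
; The box overlap casts to BP_PetitFille, and a DoOnce limits the sequence to the first entry.
; A looping index walks the Sound array, playing each entry's sound in 2D and waiting that entry's delay before advancing to the next.
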(event OnComponentBeginOverlap(Box)
  (params (OverlappedComponent :type Primitive%20Component%20Object%20Reference) (OtherActor :type Actor%20Object%20Reference) (OtherComp :type Primitive%20Component%20Object%20Reference) (OtherBodyIndex :type Integer) (bFromSweep :type Boolean) (SweepResult :type Hit%20Result%20Structure%20%28by%20ref%29))
  (bind _sound (Variables|Default|GetSound))
  (bind _index (Variables|Default|Getindex))
  (bind _output (Utilities|Array|Get(acopy) _sound _index))
  (bind (_son _delay) (Utilities|Struct|BreakStruc_ScriptSon _output))
  (Utilities|Casting|CastToBP_PetitFille OtherActor)
  (Utilities|FlowControl|DoOnce false
    (:Completed
      (if (Utilities|Array|IsValidIndex (Variables|Default|GetSound) (Variables|Default|Getindex)) :!label _label
        (Audio|PlaySound2D _son 1.0 1.0 0.0 0 0)
        (Utilities|FlowControl|Delay _delay)
        (Math|Integer|IncrementInt (Variables|Default|Getindex)
          (:%20%20
            (goto _label)))))))

(fn ConstructionScript)