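; A door Blueprint that swings open once when interacted with, optionally requiring a named item.
; The Interaction event receives an array and, when an item is required, searches it for a matching Name before opening.
; Opening plays a 2D sound, waits a configurable delay, then runs the DoorAction timeline to rotate the mesh's yaw to a set angle.
; BeginPlay sets the timeline's play rate from a speed variable.
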(event EventInteraction
  (params (Tab :type Array%20of%20Struc%20Inventory%20Structures))
  (bind _staticmesh (Variables|Default|GetStaticMesh))
  (bind _relativerotation (Variables|/Script/Engine.SceneComponent|GetRelativeRotation _staticmesh))
  ;[1 1 1] if i need a item
  (if (Variables|NeedOpen|GetneedItemBoolean)
    ;[1 1 1] verif item
    (bind _array_element (Utilities|Array|ForEachLoopwithBreak Tab :!label _label)
      (:LoopBody
        (if (== (Variables|NeedOpen|GetneedItem) (.Name (Utilities|Struct|BreakStruc_Inventory _array_element)))
          (Utilities|FlowControl|DoOnce false :!label _label_2
            (:Completed
              ;[1 1 1] open
              (Audio|PlaySound2D (Variables|sound|GetSound) 1.0 1.0 0.0 0 0)
              (Utilities|FlowControl|Delay (Variables|Sound|GetTimerSoundBeforeAnim))
              (bind _newtrack_0 (Timeline|DoorAction PlayFromStart)
                (:Update
                  (Transformation|SetRelativeRotation _staticmesh (Math|Rotator|MakeRotator (.roll _relativerotation) (.pitch _relativerotation) (Math|Float|MapRangeClamped _newtrack_0 0.0 1.0 0.0 (Variables|anim|GetAngle))) false false))
                (:Finished
                  (goto _label Break))))))))
    (else
      (goto _label_2))))

(event EventBeginPlay
  (Components|Timeline|SetPlayRate (Variables|Default|GetDoorAction) (Variables|Anim|GetSpeed)))

(fn ConstructionScript
  (|CallParentFunction))