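; BP_BalaiScript is a broom actor that falls over by itself shortly after play begins.
; After a short delay, BeginPlay calls BalaiFall and spawns a falling-broom sound at the actor's location.
; A timeline drives the actor's roll to tip it over while keeping pitch and yaw, then enables physics simulation on the mesh when it finishes.
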(event Custom|BalaiFall
  (bind _returnvalue (Transformation|GetActorRotation))
  (bind _newtrack_0 (Timeline|Timeline_0 PlayFromStart)
    (:Update
      (Transformation|SetActorRelativeRotation (Math|Rotator|MakeRotator (Math|Float|MapRangeClamped _newtrack_0 0.0 1.0 0.0 8e+01) (.pitch _returnvalue) (.yaw _returnvalue))))
    (:Finished
      (Physics|SetSimulatePhysics (Variables|Debug|GetStaticMeshComponent) true))))

(event EventBeginPlay
  (Utilities|FlowControl|Delay 3.0)
  (CallFunction|BalaiFall)
  (Audio|SpawnSoundatLocation "/Game/Audio/Wave/Kitchen/SFX_OSFallinBroom_01_GOICO__v1.SFX_OSFallinBroom_01_GOICO__v1" (Transformation|GetActorLocation) "0, 0, 0" 1.0 1.0 0.0 0 0))

(fn ConstructionScript)