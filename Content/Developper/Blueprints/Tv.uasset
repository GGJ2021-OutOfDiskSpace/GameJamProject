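; Interactive TV that starts switched off and serves as one of the lights the player has to fix.
; On begin play its spot light and mesh glow are off, the red button is lit, and its three audio sources are paused.
; The first Interaction flips both light and material Power states, resumes the audio, and decrements LightToFix on the BP_PetitFille player pawn.
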(event EventInteraction
  (params (Tab :type Array%20of%20Struc%20Inventory%20Structures))
  ;[1 1 1] Tv
  (Utilities|FlowControl|DoOnce false
    (:Completed
      (CallFunction|SetVisibilityandLight (Variables|/Script/Engine.Light|GetLightComponent (Variables|Default|Getspot)) (Variables|Default|GetStaticMesh) true)
      ;[1 1 1] BtnRed
      (CallFunction|SetVisibilityandLight (Variables|/Script/Engine.Light|GetLightComponent (Variables|Default|Getpoint)) (Variables|Default|GetCube1) false)
      (CallFunction|SetSound false)
      (bind _asbp_petit_fille (Utilities|Casting|CastToBP_PetitFille (Game|Player|GetPlayerPawn 0)))
      (Math|Integer|DecrementInt (Variables|/Game/Developper/Blueprints/BP_PetitFille.BP_PetitFille_C|GetLightToFix _asbp_petit_fille)))))

(event EventBeginPlay
  ;[1 1 1] Tv
  (CallFunction|SetVisibilityandLight (Variables|/Script/Engine.Light|GetLightComponent (Variables|Default|Getspot)) (Variables|Default|GetStaticMesh) false)
  ;[1 1 1] BtnRed
  (CallFunction|SetVisibilityandLight (Variables|/Script/Engine.Light|GetLightComponent (Variables|Default|Getpoint)) (Variables|Default|GetCube1) true)
  (CallFunction|SetSound true))

(fn ConstructionScript
  (|CallParentFunction))

(fn SetVisibilityandLight
  (params (visibilityActor :type Scene%20Component%20Object%20Reference) (powerActor :type Mesh%20Component%20Object%20Reference) (visibility :type Boolean))
  (Rendering|SetVisibility visibilityActor visibility false)
  (Rendering|Material|SetScalarParameterValueonMaterials powerActor "Power" (select visibility 1.0 0.0)))

(fn SetSound
  (params (pauseSound? :type Boolean))
  (for _array_element (Utilities|Array|MakeArray (Variables|Default|GetAudio) (Variables|Default|GetAudio1) (Variables|Default|GetAudio2))
    (Class|AudioComponent|SetPaused _array_element pauseSound?))
  (return))