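; BP_CheckLights is a trigger gate that checks whether BP_PetitFille still has lights to fix when she overlaps its collision component.
; With none left, it sets her LightToFix to NewLightFix and destroys itself.
; Otherwise it shows a WG_HudSpeak widget fed by its Speaking value, and a timeline lerps her a short distance along the Arrow's forward direction without sweep.
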(event OnComponentBeginOverlap(CollisionComponent)
  (params (OverlappedComponent :type Primitive%20Component%20Object%20Reference) (OtherActor :type Actor%20Object%20Reference) (OtherComp :type Primitive%20Component%20Object%20Reference) (OtherBodyIndex :type Integer) (bFromSweep :type Boolean) (SweepResult :type Hit%20Result%20Structure%20%28by%20ref%29))
  (bind _asbp_petit_fille (Utilities|Casting|CastToBP_PetitFille OtherActor))
  (if (== (Variables|/Game/Developper/Blueprints/BP_PetitFille.BP_PetitFille_C|GetLightToFix _asbp_petit_fille) 0)
    (bind _asbp_petit_fille_2 (Utilities|Casting|CastToBP_PetitFille (Game|Player|GetPlayerPawn 0)))
    (Variables|/Game/Developper/Blueprints/BP_PetitFille.BP_PetitFille_C|SetLightToFix _asbp_petit_fille_2 (Variables|Default|GetNewLightFix))
    (Actor|DestroyActor)
    (else
      (bind _returnvalue (UserInterface|CreateWidget "/Game/Developper/Blueprints/Widgets/WG_HudSpeak.WG_HudSpeak_C" 0 (Variables|Default|GetSpeaking)))
      (UserInterface|Viewport|AddtoViewport _returnvalue 0)
      (Variables|Default|SetActorTempLoc (Transformation|GetActorLocation _asbp_petit_fille))
      (bind _newtrack_0 (Timeline|Timeline_0 PlayFromStart)
        (:Update
          (Transformation|SetActorLocation _asbp_petit_fille (Math|Vector|Lerp(Vector) (Variables|Default|GetActorTempLoc) (+ (Variables|Default|GetActorTempLoc) (* (Math|Vector|GetForwardVector (Variables|Default|GetArrow)) 4e+01)) _newtrack_0) false false))))))

(fn ConstructionScript)