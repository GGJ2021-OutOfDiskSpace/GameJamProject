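; BP_Cine is a trigger actor that starts a video cinematic when the player character BP_PetitFille overlaps its box.
; If the character's gameplay audio is valid, the overlap pauses it, then a DoOnce disables player input.
; The same one-shot step creates a WG_VideoOpen widget with the actor's delay, sound and media source and adds it to the viewport.
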(event OnComponentBeginOverlap(Box)
  (params (OverlappedComponent :type Primitive%20Component%20Object%20Reference) (OtherActor :type Actor%20Object%20Reference) (OtherComp :type Primitive%20Component%20Object%20Reference) (OtherBodyIndex :type Integer) (bFromSweep :type Boolean) (SweepResult :type Hit%20Result%20Structure%20%28by%20ref%29))
  (bind _asbp_petit_fille (Utilities|Casting|CastToBP_PetitFille OtherActor))
  (Utilities|IsValid (Variables|/Game/Developper/Blueprints/BP_PetitFille.BP_PetitFille_C|GetAudioGameplay _asbp_petit_fille)
    (:Is%20Valid
      (Class|AudioComponent|SetPaused (Variables|/Game/Developper/Blueprints/BP_PetitFille.BP_PetitFille_C|GetAudioGameplay _asbp_petit_fille) true)
      (Utilities|FlowControl|DoOnce false
        (:Completed
          (Input|DisableInput _asbp_petit_fille (Game|GetPlayerController 0))
          (bind _returnvalue (UserInterface|CreateWidget "/Game/Developper/Blueprints/Widgets/WG_VideoOpen.WG_VideoOpen_C" 0 false (Variables|Default|GetDelay) (Variables|Default|GetSD) (Variables|Default|GetVideo)))
          (UserInterface|Viewport|AddtoViewport _returnvalue 0))))))

(fn ConstructionScript)