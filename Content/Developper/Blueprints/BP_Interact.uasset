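; BP_Interact is an interactable actor built around a configurable static mesh, with an empty Interaction event that takes a Tab parameter.
; The construction script applies the Mesh and Material variables to the StaticMesh component.
; RenderDepthON and RenderDepthOFF toggle the mesh's custom depth rendering, gated by the HasRender flag.
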(event Custom|Render%20Depth%20OFF
  (if (Variables|Default|GetHasRender)
    (Rendering|SetRenderCustomDepth (Variables|Default|GetStaticMesh) false)))

(event Custom|Render%20Depth%20ON
  (if (Variables|Default|GetHasRender)
    (Rendering|SetRenderCustomDepth (Variables|Default|GetStaticMesh) true)))

(event Custom|Interaction
  (params (Tab :type Array%20of%20Struc%20Inventory%20Structures)))

(fn ConstructionScript
  (bind _staticmesh (Variables|Default|GetStaticMesh))
  (Components|StaticMesh|SetStaticMesh _staticmesh (Variables|Default|GetMesh))
  (Rendering|Material|SetMaterial _staticmesh 0 (Variables|Default|GetMaterial)))