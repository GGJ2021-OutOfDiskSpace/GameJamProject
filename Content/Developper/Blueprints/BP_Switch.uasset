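; BP_Switch is a one-use interactable light switch that turns on its referenced point and spot lights.
; On BeginPlay it hides those lights; the first Interaction plays a click sound, flips the button mesh via negative Z scale and makes them visible.
; It also triggers the optional broom-fall script (BalaiFall) and decrements the LightToFix counter on the BP_PetitFille player pawn.
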(event EventBeginPlay
  (for _array_element (Variables|Default|GetpointLight)
    (Rendering|SetVisibility (Variables|/Script/Engine.Light|GetLightComponent _array_element) false false))
  (for _array_element_2 (Variables|Default|GetspotLight)
    (Rendering|SetVisibility (Variables|/Script/Engine.SpotLight|GetSpotLightComponent _array_element_2) false false)))

(event EventInteraction
  (params (Tab :type Array%20of%20Struc%20Inventory%20Structures))
  (Utilities|FlowControl|DoOnce false
    (:Completed
      (Audio|PlaySound2D "/Game/Audio/SC/SC_SwitchLight.SC_SwitchLight" 1.0 1.0 0.0 0 0)
      (bind _refbalaiscript (Variables|Default|GetRefBalaiScript)
        (:then
          (Default|BalaiFall _refbalaiscript))
        (:else
          _))
      (Transformation|SetWorldScale3D (Variables|Default|Getinterupteur_Btn) "1.000000,1.000000,-1.000000")
      (for _array_element (Variables|Default|GetpointLight)
        (Rendering|SetVisibility (Variables|/Script/Engine.Light|GetLightComponent _array_element) true false))
      (for _array_element_2 (Variables|Default|GetspotLight)
        (Rendering|SetVisibility (Variables|/Script/Engine.SpotLight|GetSpotLightComponent _array_element_2) true false))
      (bind _asbp_petit_fille (Utilities|Casting|CastToBP_PetitFille (Game|Player|GetPlayerPawn 0)))
      (Math|Integer|DecrementInt (Variables|/Game/Developper/Blueprints/BP_PetitFille.BP_PetitFille_C|GetLightToFix _asbp_petit_fille)))))

(fn ConstructionScript
  (|CallParentFunction))