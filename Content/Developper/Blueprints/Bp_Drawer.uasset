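; Interactable drawer that slides open once when its Interaction event fires.
; A Use flag blocks repeat triggers, so the Blueprint has no closing path.
; The first interaction plays a wooden drawer sound at the actor's location and starts the OuvertureTiroir timeline, which drives the static mesh's relative X position while keeping Y and Z.
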(event EventInteraction
  (params (Tab :type Array%20of%20Struc%20Inventory%20Structures))
  (bind _staticmesh (Variables|Default|GetStaticMesh))
  (bind _relativelocation (Variables|/Script/Engine.SceneComponent|GetRelativeLocation _staticmesh))
  (if (not (Variables|Default|GetUse?))
    (Variables|Default|SetUse? true)
    (Audio|PlaySoundatLocation "/Game/Audio/SC/SC_WoodenDrawerOpen.SC_WoodenDrawerOpen" (Transformation|GetActorLocation) "0, 0, 0" 1.0 1.0 0.0 0 0 0)
    (bind _newtrack_0 (Timeline|ouvertureTiroir PlayFromStart)
      (:Update
        (Transformation|SetRelativeLocation _staticmesh (Math|Vector|MakeVector _newtrack_0 (.y _relativelocation) (.z _relativelocation)) false false)))))

(fn ConstructionScript
  (|CallParentFunction))