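; Pushable box that the BP_PetitFille player character moves through physics, with a configurable mass (Poids).
; Interaction enables physics and frees the PhysicsConstraint's linear X/Y axes.
; Each Tick while the player holds interact and can push, a short sphere trace along their facing direction disables physics if blocked.
; A moving sound plays while the path is clear; releasing or losing push ability stops it and disables physics.
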(event EventBeginPlay
  (bind _poids (Variables|Default|GetPoids))
  (Class|PrimitiveComponent|SetAllMassScale (Variables|Default|GetStaticMesh) _poids)
  (Class|PrimitiveComponent|SetMassOverrideinKg (Variables|Default|GetStaticMesh) "None" _poids true))

(event EventInteraction
  (params (Tab :type Array%20of%20Struc%20Inventory%20Structures))
  (bind _physicsconstraint (Variables|Default|GetPhysicsConstraint))
  (Physics|SetSimulatePhysics (Variables|Default|GetStaticMesh) true)
  (Class|PhysicsConstraintComponent|SetLinearXLimit _physicsconstraint "LCM_Free" 0.0)
  (Class|PhysicsConstraintComponent|SetLinearYLimit _physicsconstraint "LCM_Free" 0.0))

(event EventTick
  (params (DeltaSeconds :type Float%20%28single-precision%29))
  (bind _staticmesh (Variables|Default|GetStaticMesh))
  (bind _returnvalue (Transformation|GetWorldLocation _staticmesh))
  (bind (_x _y _z) (Math|Vector|BreakVector _returnvalue))
  ;[1 1 1] Comment
  (bind _asbp_petit_fille (Utilities|Casting|CastToBP_PetitFille (Game|Player|GetPlayerPawn 0)))
  (if (Variables|/Game/Developper/Blueprints/BP_PetitFille.BP_PetitFille_C|GetHoldingInteract? _asbp_petit_fille)
    (if (Variables|/Game/Developper/Blueprints/BP_PetitFille.BP_PetitFille_C|GetCanPush _asbp_petit_fille)
      (bind _asbp_petit_fille_2 (Utilities|Casting|CastToBP_PetitFille (Game|Player|GetPlayerPawn 0)))
      (Utilities|IsValid (Variables|Default|GetMovingObjectSound)
        (:Is%20Valid
          _)
        (:Is%20Not%20Valid
          (bind _returnvalue_2 (Audio|CreateSound2D (Variables|Default|GetSoundToPlay) 1.0 1.0 0.0 0))
          (Variables|Default|SetMovingObjectSound _returnvalue_2)))
      (bind _returnvalue_3 (Collision|SphereTraceByChannel (Math|Vector|MakeVector _x _y (+ _z 2e+01)) (Math|Vector|MakeVector (.x (+ _returnvalue (* (Math|Vector|GetForwardVector (Variables|/Script/Engine.Character|GetCapsuleComponent _asbp_petit_fille_2)) 5e+01))) (.y (+ _returnvalue (* (Math|Vector|GetForwardVector (Variables|/Script/Engine.Character|GetCapsuleComponent _asbp_petit_fille_2)) 5e+01))) (+ (.z (+ _returnvalue (* (Math|Vector|GetForwardVector (Variables|/Script/Engine.Character|GetCapsuleComponent _asbp_petit_fille_2)) 5e+01))) 2e+01)) 15.0 "TraceTypeQuery1" false 0 "None"))
      (Physics|SetSimulatePhysics (Variables|Default|GetStaticMesh) (not _returnvalue_3))
      (if (not _returnvalue_3)
        (if (not (Audio|Components|Audio|IsPlaying (Variables|Default|GetMovingObjectSound)))
          (Audio|Components|Audio|Play (Variables|Default|GetMovingObjectSound) 0.0))
        (elif (Audio|Components|Audio|IsPlaying (Variables|Default|GetMovingObjectSound))
          (Audio|Components|Audio|Stop (Variables|Default|GetMovingObjectSound))))
      (else
        (Physics|SetSimulatePhysics (Variables|Default|GetStaticMesh) false :!label _label)
        (Variables|Default|SetActivated false)
        (Utilities|IsValid (Variables|Default|GetMovingObjectSound)
          (:Is%20Valid
            (if (Audio|Components|Audio|IsPlaying (Variables|Default|GetMovingObjectSound))
              (Audio|Components|Audio|Stop (Variables|Default|GetMovingObjectSound)))))))
    (else
      (goto _label))))

(fn ConstructionScript
  (|CallParentFunction))