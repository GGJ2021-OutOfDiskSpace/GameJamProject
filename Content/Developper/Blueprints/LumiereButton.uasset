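; LumiereButton is an interactable button that switches on an assigned set of lights.
; At BeginPlay it hides the light component of every entry in its Light array.
; Its Interaction event fires once through a DoOnce, makes those lights visible, then decrements the NbLumiere counter on the player's BP_PetitFille pawn.
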(event EventInteraction
  (params (Tab :type Array%20of%20Struc%20Inventory%20Structures))
  (Utilities|FlowControl|DoOnce false
    (:Completed
      (for _array_element (Variables|Default|Getlight)
        (Rendering|SetVisibility (Variables|/Script/Engine.Light|GetLightComponent _array_element) true false))
      (bind _asbp_petit_fille (Utilities|Casting|CastToBP_PetitFille (Game|Player|GetPlayerPawn 0)))
      (Math|Integer|DecrementInt (Variables|/Game/Developper/Blueprints/BP_PetitFille.BP_PetitFille_C|GetnbLumiere _asbp_petit_fille)))))

(event EventBeginPlay
  (for _array_element (Variables|Default|Getlight)
    (Rendering|SetVisibility (Variables|/Script/Engine.Light|GetLightComponent _array_element) false false)))

(fn ConstructionScript
  (|CallParentFunction))