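; Wall-switch style interactable ("Interupteur") whose button visually flips when the little-girl player, BP_PetitFille, uses it.
; Every Tick it polls the player pawn, checking that its InteractObject is this actor and HoldingInteract is set.
; A DoOnce with no reset then mirrors InterupteurBtn on Z through a negative world scale, so the flip happens only once and triggers nothing else here.
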(event EventTick
  (params (DeltaSeconds :type Float%20%28single-precision%29))
  (bind _returnvalue (Game|Player|GetPlayerPawn 0))
  (bind _asbp_petit_fille (Utilities|Casting|CastToBP_PetitFille _returnvalue))
  (if (and (== (Variables|/Game/Developper/Blueprints/BP_PetitFille.BP_PetitFille_C|GetInteractObject _asbp_petit_fille) self) (Variables|/Game/Developper/Blueprints/BP_PetitFille.BP_PetitFille_C|GetHoldingInteract? _asbp_petit_fille))
    (Utilities|FlowControl|DoOnce false
      (:Completed
        (Transformation|SetWorldScale3D (Variables|Default|Getinterupteur_Btn) "1.000000,1.000000,-1.000000")))))

(fn ConstructionScript
  (|CallParentFunction))