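; BP_Preview is an interactable slot where the player places the inventory item whose name matches its own.
; On a first match it plays a sound and, if the item has a valid mesh, switches collision from Visibility to WorldDynamic, takes on that mesh and its materials, and removes the item from BP_PetitFille's inventory.
; The "Frog" item additionally slides into place through one timeline, then a second drives a point light's intensity.
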(event EventBeginPlay
  (Collision|SetCollisionObjectType (Variables|Default|GetStaticMesh) "ECC_Visibility"))

(event EventInteraction
  (params (Tab :type Array%20of%20Struc%20Inventory%20Structures))
  (bind _previewanimation (Variables|Default|GetPreviewAnimation))
  (bind _staticmesh (Variables|Default|GetStaticMesh))
  (bind _relativelocation (Variables|/Script/Engine.SceneComponent|GetRelativeLocation _previewanimation))
  (bind (_array_element _array_index) (Utilities|Array|ForEachLoopwithBreak Tab :!label _label)
    (:LoopBody
      (if (not (Variables|Default|GetUse))
        (if (Utilities|Enum|Equal(Enum) (.Name (Utilities|Struct|BreakStruc_Inventory _array_element)) (Variables|Default|GetName))
          (Audio|PlaySound2D (Variables|Default|GetSound) 1.0 1.0 0.0 0 0)
          (Utilities|IsValid (.Mesh (Utilities|Struct|BreakStruc_Inventory _array_element))
            (:Is%20Valid
              (Variables|Default|SetUse true)
              (Collision|SetCollisionObjectType (Variables|Default|GetStaticMesh) "ECC_WorldDynamic")
              (for (_ _array_index_2) (Rendering|Material|GetMaterials (Variables|Default|GetStaticMesh))
                (Rendering|Material|SetMaterial _staticmesh _array_index_2 (Rendering|Material|GetMaterial (.Mesh (Utilities|Struct|BreakStruc_Inventory _array_element)) _array_index_2)))
              (Components|StaticMesh|SetStaticMesh _staticmesh (.Mesh (Utilities|Struct|BreakStruc_Inventory _array_element)))
              (bind _asbp_petit_fille (Utilities|Casting|CastToBP_PetitFille (Game|Player|GetPlayerPawn 0)))
              (Utilities|Array|RemoveIndex (Variables|/Game/Developper/Blueprints/BP_PetitFille.BP_PetitFille_C|Getinventory _asbp_petit_fille) _array_index)
              (if (Utilities|Enum|Equal(Enum) (Variables|Default|GetName) (Utilities|Text|FormatText "Frog"))
                (Transformation|SetRelativeLocation (Variables|Default|GetStaticMesh) _relativelocation false false)
                (bind _alpha (Timeline|Timeline_0 PlayFromStart)
                  (:Update
                    (Transformation|SetRelativeLocation (Variables|Default|GetStaticMesh) (Math|Vector|Lerp(Vector) _relativelocation "0, 0, 0" _alpha) false false))
                  (:Finished
                    (bind _intensity (Timeline|Timeline_1 PlayFromStart)
                      (:Update
                        (Rendering|Components|Light|SetIntensity (Variables|Default|GetPointLight) (Math|Float|MapRangeClamped _intensity 0.0 1.0 0.0 (Variables|Default|GetFrogLightIntensity))))
                      (:Finished
                        (goto _label Break)))))
                (else
                  (goto _label Break))))))))))

(fn ConstructionScript
  (|CallParentFunction))