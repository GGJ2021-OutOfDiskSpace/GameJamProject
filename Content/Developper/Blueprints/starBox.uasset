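; starBox is a trigger actor that removes a blocking actor when the little girl character, BP_PetitFille, overlaps it with a star.
; On overlap it only proceeds if her NbLumiere count is zero, otherwise it prints a fear-of-the-dark message.
; It then scans her Inventory for an item named "star" and destroys the Blocking actor if found, or prints that she lacks her star.
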(event Collision|EventActorBeginOverlap
  (params (OtherActor :type Actor%20Object%20Reference))
  (bind _blocking (Variables|Default|Getblocking))
  (bind _asbp_petit_fille (Utilities|Casting|CastToBP_PetitFille OtherActor))
  (if (== (Variables|/Game/Developper/Blueprints/BP_PetitFille.BP_PetitFille_C|GetnbLumiere _asbp_petit_fille) 0)
    (Variables|Default|Setstar? false)
    (for _array_element (Variables|/Game/Developper/Blueprints/BP_PetitFille.BP_PetitFille_C|Getinventory _asbp_petit_fille)
      (if (Utilities|Enum|Equal(Enum) (.Name (Utilities|Struct|BreakStruc_Inventory _array_element)) (Utilities|Text|MakeLiteralText "star"))
        (Variables|Default|Setstar? true)))
    (if (Variables|Default|Getstar?)
      (Utilities|IsValid _blocking
        (:Is%20Valid
          (Actor|DestroyActor _blocking)))
      (else
        (Development|PrintString "j'ai pas mon etoile")))
    (else
      (Development|PrintString "j'ai peur du noir"))))

(fn ConstructionScript)