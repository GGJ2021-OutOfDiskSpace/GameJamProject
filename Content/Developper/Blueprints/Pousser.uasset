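; Pushable object that the player (BP_PetitFille) moves while holding interact on it.
; Each Tick, the cone macro fans debug-drawn sphere traces from the mesh around the player's forward vector, and any hit blocks the push.
; If the path is clear and the player roughly lines up on world X or Y, the mesh steps away along the other axis, one unit per frame without sweep.
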(event EventTick
  (params (DeltaSeconds :type Float%20%28single-precision%29))
  (bind _returnvalue (Game|Player|GetPlayerPawn 0))
  (bind _returnvalue_2 (Game|Player|GetPlayerPawn 0))
  (bind _returnvalue_3 (Game|Player|GetPlayerPawn 0))
  (bind _staticmesh (Variables|Default|GetStaticMesh))
  (bind _staticmesh_2 (Variables|Default|GetStaticMesh))
  (bind _returnvalue_4 (Transformation|GetWorldLocation _staticmesh_2))
  (bind _returnvalue_5 (Transformation|GetWorldLocation _staticmesh))
  (bind _asbp_petit_fille (Utilities|Casting|CastToBP_PetitFille _returnvalue))
  (bind _asbp_petit_fille_2 (Utilities|Casting|CastToBP_PetitFille _returnvalue_2))
  (bind _asbp_petit_fille_3 (Utilities|Casting|CastToBP_PetitFille _returnvalue_3))
  (bind _capsulecomponent (Variables|/Script/Engine.Character|GetCapsuleComponent _asbp_petit_fille_3))
  (bind _capsulecomponent_2 (Variables|/Script/Engine.Character|GetCapsuleComponent _asbp_petit_fille_2))
  (bind _returnvalue_6 (Transformation|GetWorldLocation _capsulecomponent_2))
  (bind _returnvalue_7 (Transformation|GetWorldLocation _capsulecomponent))
  (bind _returnvalue_8 (Math|Float|NearlyEqual(Float) (.x _returnvalue_7) (.x _returnvalue_5) 5e+01))
  (if (and (== (Variables|/Game/Developper/Blueprints/BP_PetitFille.BP_PetitFille_C|GetInteractObject _asbp_petit_fille) self) (Variables|/Game/Developper/Blueprints/BP_PetitFille.BP_PetitFille_C|GetHoldingInteract? _asbp_petit_fille))
    (Variables|Default|Setis%20valid? true)
    ;[1 1 1] isAngleValid
    (bind _newparam (Utilities|Cone 1e+01 1e+01 :!label _label)
      (:enCours
        (if _newparam
          (Variables|Default|Setis%20valid? false)
          (goto _label break)))
      (:completed
        (if (Variables|Default|Getis%20valid?)
          (if (or _returnvalue_8 (Math|Float|NearlyEqual(Float) (.y _returnvalue_7) (.y _returnvalue_5) 5e+01))
            (if _returnvalue_8
              (Transformation|SetWorldLocation (Variables|Default|GetStaticMesh) (+ (Transformation|GetWorldLocation (Variables|Default|GetStaticMesh)) (select (> (.y _returnvalue_6) (.y _returnvalue_4)) "0,-1.000000, 0" "0,1.000000, 0")) false false)
              (else
                (Transformation|SetWorldLocation (Variables|Default|GetStaticMesh) (+ (Transformation|GetWorldLocation (Variables|Default|GetStaticMesh)) (select (> (.x _returnvalue_6) (.x _returnvalue_4)) "-1.000000,0.000000, 0" "1.000000,0.000000, 0")) false false)))))))))

(fn ConstructionScript
  (|CallParentFunction))